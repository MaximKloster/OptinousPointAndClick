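; BP_Player_Scaler is a Blueprint that resizes itself to match the height of the player tracked by a Kinect sensor.
; Each tick it gets the centered body and, if tracked, estimates player size by summing torso, right leg and doubled head-to-neck joint distances.
; That size, divided by a fixed reference, sets the root's world scale on Y and Z, leaving X unscaled.
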(event EventBeginPlay)

(event EventActorBeginOverlap
  (params (OtherActor :type Actor%20Object%20Reference)))

(event EventTick
  (params (DeltaSeconds :type Float%20%28single-precision%29))
  (bind _kinectinterface (Variables|Default|GetKinectInterface))
  (bind (_centeredbody _istracked) (Class|KinectInterfaceComponent|GetCenteredBody _kinectinterface))
  (if _istracked
    (bind _returnvalue (Class|KinectInterfaceComponent|GetDistanceBetweenJoints _kinectinterface "Neck" "SpineBase" _centeredbody))
    (bind _returnvalue_2 (Class|KinectInterfaceComponent|GetDistanceBetweenJoints _kinectinterface "FootRight" "SpineBase" _centeredbody))
    (bind _returnvalue_3 (Class|KinectInterfaceComponent|GetDistanceBetweenJoints _kinectinterface "Head" "Neck" _centeredbody))
    (Variables|Default|SetPlayerSize (+ _returnvalue _returnvalue_2 (* _returnvalue_3 2.0)))
    (Transformation|SetWorldScale3D (Variables|Default|Getroot) (Math|Vector|MakeVector 1.0 (/ (Variables|Default|GetPlayerSize) 2e+02) (/ (Variables|Default|GetPlayerSize) 2e+02)))))

(fn ConstructionScript)