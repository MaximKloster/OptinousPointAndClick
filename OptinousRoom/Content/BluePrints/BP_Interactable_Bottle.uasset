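; Bottle interactable that a KinectCharacter picks up and releases through tracked hand states.
; Trigger overlap matches hand collision tags and, for a hand in state 2, disables the bottle's physics and collision.
; Tick snaps it to the hand's middle-finger socket on state 3 and detaches it with physics restored on state 2.
; Left-hand overlap sets its interaction flag false, so left-hand pickup never triggers.
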(event OnComponentEndOverlap(Trigger)
  (params (OtherActor :type Actor%20Object%20Reference) (OtherComp :type Primitive%20Component%20Object%20Reference) (OtherBodyIndex :type Integer))
  (bind _bottle (Variables|Default|GetBottle))
  (if (not (Variables|Default|GetIsInRightHand))
    (if (not (Variables|Default|GetIsInLeftHand))
      (Variables|Default|SetIsInInteractionLeft false)
      (Variables|Default|SetIsInInteractionRight false)
      (Collision|SetCollisionEnabled _bottle "QueryAndPhysics")
      (Physics|SetSimulatePhysics _bottle true))))

(event OnComponentBeginOverlap(Trigger)
  (params (OtherActor :type Actor%20Object%20Reference) (OtherComp :type Primitive%20Component%20Object%20Reference) (OtherBodyIndex :type Integer) (bFromSweep :type Boolean) (SweepResult :type Hit%20Result%20Structure%20%28by%20ref%29))
  (bind _bottle (Variables|Default|GetBottle))
  ;[1 1 1] Which Hand is in Interaction Area of the Object, deactivate the Collision of the Object
  (bind _askinect_character (Utilities|Casting|CastToKinectCharacter OtherActor))
  (for _array_element (Variables|/Script/Engine.ActorComponent|GetComponentTags OtherComp)
    (if (Utilities|Name|Equal(Name) _array_element (Variables|/Game/Blueprints/KinectCharacter.KinectCharacter_C|GetRightHandCollisionTag _askinect_character))
      (if (== (Variables|/Game/Blueprints/KinectCharacter.KinectCharacter_C|GetRightHandState _askinect_character) 2)
        (Variables|Default|SetIsInInteractionRight true)
        (Physics|SetSimulatePhysics _bottle false :!label _label)
        (Collision|SetCollisionEnabled _bottle "NoCollision"))
      (elif (Utilities|Name|Equal(Name) _array_element (Variables|/Game/Blueprints/KinectCharacter.KinectCharacter_C|GetLeftHandCollisionTag _askinect_character))
        (if (== (Variables|/Game/Blueprints/KinectCharacter.KinectCharacter_C|GetLeftHandState _askinect_character) 2)
          (Variables|Default|SetIsInInteractionLeft false)
          (goto _label))))))

(event EventBeginPlay)

(event EventActorBeginOverlap
  (params (OtherActor :type Actor%20Object%20Reference)))

(event EventTick
  (params (DeltaSeconds :type Float%20%28single-precision%29))
  (bind _bottle (Variables|Default|GetBottle))
  (bind _bottle_2 (Variables|Default|GetBottle))
  (if (Variables|Default|GetIsInInteractionRight)
    (if (== (Variables|/Game/Blueprints/KinectCharacter.KinectCharacter_C|GetRightHandState (stale OnComponentBeginOverlap(Trigger) _askinect_character)) 3)
      (Variables|Default|SetIsInInteractionRight false)
      (Class|SceneComponent|Attachto _bottle (Variables|/Game/Blueprints/KinectCharacter.KinectCharacter_C|GetKinectMesh (stale OnComponentBeginOverlap(Trigger) _askinect_character)) "middle_01_r" "SnapToTarget" true)
      (Variables|Default|SetIsInRightHand true))
    (elif (Variables|Default|GetIsInInteractionLeft)
      (if (== (Variables|/Game/Blueprints/KinectCharacter.KinectCharacter_C|GetLeftHandState (stale OnComponentBeginOverlap(Trigger) _askinect_character)) 3)
        (Variables|Default|SetIsInInteractionLeft false)
        (Class|SceneComponent|Attachto _bottle (Variables|/Game/Blueprints/KinectCharacter.KinectCharacter_C|GetKinectMesh (stale OnComponentBeginOverlap(Trigger) _askinect_character)) "middle_01_l" "SnapToTarget" true)
        (Variables|Default|SetIsInLeftHand true))
      (elif (Variables|Default|GetIsInRightHand)
        (if (== (Variables|/Game/Blueprints/KinectCharacter.KinectCharacter_C|GetRightHandState (stale OnComponentBeginOverlap(Trigger) _askinect_character)) 2)
          (Variables|Default|SetIsInRightHand false)
          (Class|SceneComponent|DetachfromParent _bottle_2 false :!label _label)
          (Collision|SetCollisionEnabled _bottle_2 "QueryAndPhysics")
          (Physics|SetSimulatePhysics _bottle_2 true))
        (elif (Variables|Default|GetIsInLeftHand)
          (if (== (Variables|/Game/Blueprints/KinectCharacter.KinectCharacter_C|GetLeftHandState (stale OnComponentBeginOverlap(Trigger) _askinect_character)) 2)
            (Variables|Default|SetIsInLeftHand false)
            (goto _label)))))))

(fn ConstructionScript)