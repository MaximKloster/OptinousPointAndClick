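; Actor that displays live Kinect RGB, infrared and depth camera feeds on three in-world screens.
; On BeginPlay it fetches each camera frame texture from the Kinect interface and feeds it into a separate dynamic material instance on each screen.
; RGB goes to the big screen, while IR and depth go to the two right-hand screens.
; It then enables frame updating for all three cameras, so no Tick logic is used.
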(event EventBeginPlay
  (bind _kinectinterface (Variables|Default|GetKinectInterface))
  ;[1 1 1] Set dynamic material with the kinect cameras as texture
  (bind _returnvalue (Class|KinectInterfaceComponent|GetCameraFrame _kinectinterface "RGB"))
  (bind _returnvalue_2 (Rendering|Material|CreateDynamicMaterialInstance (Variables|Default|GetBigScreen) 0 "/Game/Materials/Dynamic_Material.Dynamic_Material" :!class /Script/Engine.PrimitiveComponent))
  (Rendering|Material|SetTextureParameterValue _returnvalue_2 "None" _returnvalue)
  (bind _returnvalue_3 (Class|KinectInterfaceComponent|GetCameraFrame _kinectinterface "IR"))
  (bind _returnvalue_4 (Rendering|Material|CreateDynamicMaterialInstance (Variables|Default|GetTopRightScreen) 0 "/Game/Materials/Dynamic_Material.Dynamic_Material" :!class /Script/Engine.PrimitiveComponent))
  (Rendering|Material|SetTextureParameterValue _returnvalue_4 "None" _returnvalue_3)
  (bind _returnvalue_5 (Class|KinectInterfaceComponent|GetCameraFrame _kinectinterface "Depth"))
  (bind _returnvalue_6 (Rendering|Material|CreateDynamicMaterialInstance (Variables|Default|GetBorRightScreen) 0 "/Game/Materials/Dynamic_Material.Dynamic_Material" :!class /Script/Engine.PrimitiveComponent))
  (Rendering|Material|SetTextureParameterValue _returnvalue_6 "None" _returnvalue_5)
  ;[1 1 1] Update the camera views
  (Class|KinectInterfaceComponent|SetCameraFrameIsUpdating _kinectinterface "RGB" true)
  (Class|KinectInterfaceComponent|SetCameraFrameIsUpdating _kinectinterface "IR" true)
  (Class|KinectInterfaceComponent|SetCameraFrameIsUpdating _kinectinterface "Depth" true))

(event EventActorBeginOverlap
  (params (OtherActor :type Actor%20Object%20Reference)))

(event EventTick
  (params (DeltaSeconds :type Float%20%28single-precision%29)))

(fn ConstructionScript)