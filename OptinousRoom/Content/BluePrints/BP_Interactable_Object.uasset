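; Interactable bottle actor that a Kinect-driven character can grab and throw with either hand.
; Trigger overlap with a tagged hand in state 2 disables the bottle's physics and collision; Tick attaches it to the middle-finger socket at state 3.
; While held, a rolling six-sample position history is recorded.
; Returning to state 2 detaches it, restores physics and applies force scaled from the oldest-to-newest displacement.
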(event OnComponentEndOverlap(Trigger)
  (params (OtherActor :type Actor%20Object%20Reference) (OtherComp :type Primitive%20Component%20Object%20Reference) (OtherBodyIndex :type Integer))
  ;[1 1 1] A Player Hand is not more in the Interaction Range
  (CallFunction|CheckHand OtherActor OtherComp)
  (if (not (Variables|Default|GetIsInRightHand))
    (if (not (Variables|Default|GetIsInLeftHand))
      (if (== (Variables|Default|GetHand) 1)
        _))))

(event OnComponentBeginOverlap(Trigger)
  (params (OtherActor :type Actor%20Object%20Reference) (OtherComp :type Primitive%20Component%20Object%20Reference) (OtherBodyIndex :type Integer) (bFromSweep :type Boolean) (SweepResult :type Hit%20Result%20Structure%20%28by%20ref%29))
  (bind _bottle (Variables|Default|GetBottle))
  ;[1 1 1] A Player Hand is in Interaction Range of the Object, deactivate Collision for possible interaction
  (CallFunction|CheckHand OtherActor OtherComp)
  (if (== (Variables|Default|GetHand) 1)
    (if (Variables|Default|GetIsInInteractionRight)
      (Physics|SetSimulatePhysics _bottle false :!label _label)
      (Collision|SetCollisionEnabled _bottle "NoCollision"))
    (elif (Variables|Default|GetIsInInteractionLeft)
      (goto _label))))

(event EventBeginPlay)

(event EventActorBeginOverlap
  (params (OtherActor :type Actor%20Object%20Reference)))

(event EventTick
  (params (DeltaSeconds :type Float%20%28single-precision%29))
  (bind _player (Variables|Default|GetPlayer))
  (bind _bottle (Variables|Default|GetBottle))
  (bind _kinectmesh (Variables|/Game/Blueprints/KinectCharacter.KinectCharacter_C|GetKinectMesh _player))
  (bind _lefthandstate (Variables|/Game/Blueprints/KinectCharacter.KinectCharacter_C|GetLeftHandState _player))
  (bind _righthandstate (Variables|/Game/Blueprints/KinectCharacter.KinectCharacter_C|GetRightHandState _player))
  ;[1 1 1] Object was picked Up by a Hand
  (if (Variables|Default|GetIsInInteractionRight)
    (if (== _righthandstate 3)
      (Variables|Default|SetIsInInteractionRight false)
      (Class|SceneComponent|Attachto _bottle _kinectmesh "middle_01_r" "SnapToTarget" true)
      (Variables|Default|SetIsInRightHand true)
      (bind _outposition (Class|SkinnedMeshComponent|TransformfromBoneSpace _kinectmesh "middle_01_r" "0, 0, 0" "0, 0, 0"))
      (Variables|Default|SetHoldingHandPositionsRight (Utilities|Array|MakeArray _outposition))
      (else
        (if (Variables|Default|GetIsInInteractionLeft) :!label _label
          (if (== _lefthandstate 3)
            (Variables|Default|SetIsInInteractionLeft false)
            (Class|SceneComponent|Attachto _bottle _kinectmesh "middle_01_l" "SnapToTarget" true)
            (Variables|Default|SetIsInLeftHand true)
            (bind _outposition_2 (Class|SkinnedMeshComponent|TransformfromBoneSpace _kinectmesh "middle_01_l" "0, 0, 0" "0, 0, 0"))
            (Variables|Default|SetHoldingHandPositionsLeft (Utilities|Array|MakeArray _outposition_2)))
          (elif (Variables|Default|GetIsInRightHand)
            (bind _charakter (CallFunction|ObjectWayinHand "Right" _player))
            (if (== _righthandstate 2)
              (CallFunction|ThrowObject "Right" _charakter 1e+02))
            (elif (Variables|Default|GetIsInLeftHand)
              (bind _charakter_2 (CallFunction|ObjectWayinHand "Left" _player))
              (if (== _lefthandstate 2)
                (CallFunction|ThrowObject "Left" _charakter_2 1e+02)))))))
    (else
      (goto _label))))

(fn ConstructionScript)

(fn CheckHand
  (params (Actor :type Actor%20Object%20Reference) (ActorComponent :type Actor%20Component%20Object%20Reference))
  (bind _askinect_character (Utilities|Casting|CastToKinectCharacter Actor))
  (Variables|Default|SetPlayer _askinect_character)
  (for _array_element (Variables|/Script/Engine.ActorComponent|GetComponentTags ActorComponent)
    (if (Utilities|Name|Equal(Name) _array_element (Variables|/Game/Blueprints/KinectCharacter.KinectCharacter_C|GetRightHandCollisionTag _askinect_character))
      (Variables|Default|SetHand "Right")
      (if (== (Variables|/Game/Blueprints/KinectCharacter.KinectCharacter_C|GetRightHandState _askinect_character) 2)
        (Variables|Default|SetIsInInteractionRight true)
        (else
          (Variables|Default|SetIsInInteractionRight false)))
      (elif (Utilities|Name|Equal(Name) _array_element (Variables|/Game/Blueprints/KinectCharacter.KinectCharacter_C|GetLeftHandCollisionTag _askinect_character))
        (Variables|Default|SetHand "Left")
        (if (== (Variables|/Game/Blueprints/KinectCharacter.KinectCharacter_C|GetLeftHandState _askinect_character) 2)
          (Variables|Default|SetIsInInteractionLeft true)
          (else
            (Variables|Default|SetIsInInteractionLeft false)))))))

(fn ThrowObject
  (params (Hand :type EHands%20Enum :default "Left") (Player :type Kinect%20Character%20Object%20Reference) (ForceFactor :type Float%20%28single-precision%29))
  (bind _kinectmesh (Variables|/Game/Blueprints/KinectCharacter.KinectCharacter_C|GetKinectMesh Player))
  (bind _bottle (Variables|Default|GetBottle))
  (bind _holdinghandpositionsright (Variables|Default|GetHoldingHandPositionsRight))
  (bind _holdinghandpositionsleft (Variables|Default|GetHoldingHandPositionsLeft))
  (bind _bottle_2 (Variables|Default|GetBottle))
  (Class|SceneComponent|DetachfromParent _bottle false)
  (if (== Hand 1)
    ;[1 1 1] Throw Object from Right Hand
    (Variables|Default|SetIsInRightHand false)
    (bind (_outposition _outrotation) (Class|SkinnedMeshComponent|TransformfromBoneSpace _kinectmesh "middle_01_r" "0, 0, 0" "0, 0, 0"))
    (Transformation|SetWorldLocationAndRotation _bottle _outposition _outrotation false)
    (Collision|SetCollisionEnabled _bottle "QueryAndPhysics")
    (Physics|SetSimulatePhysics _bottle true)
    (CallFunction|CalculateForce (Utilities|Array|Get(acopy) _holdinghandpositionsright) (Utilities|Array|Get(acopy) _holdinghandpositionsright (- (Utilities|Array|Length _holdinghandpositionsright) 1)) ForceFactor)
    (Physics|AddForce _bottle (Variables|Default|GetThrowingForce) "None")
    (else
      ;[1 1 1] Throw Object from Left Hand
      (Variables|Default|SetIsInRightHand false)
      (bind (_outposition_2 _outrotation_2) (Class|SkinnedMeshComponent|TransformfromBoneSpace _kinectmesh "middle_01_l" "0, 0, 0" "0, 0, 0"))
      (Transformation|SetWorldLocationAndRotation _bottle_2 _outposition_2 _outrotation_2 false)
      (Collision|SetCollisionEnabled _bottle_2 "QueryAndPhysics")
      (Physics|SetSimulatePhysics _bottle_2 true)
      (CallFunction|CalculateForce (Utilities|Array|Get(acopy) _holdinghandpositionsleft) (Utilities|Array|Get(acopy) _holdinghandpositionsleft (- (Utilities|Array|Length _holdinghandpositionsleft) 1)) ForceFactor)
      (Physics|AddForce _bottle_2 (Variables|Default|GetThrowingForce) "None"))))

(fn CalculateForce
  (params (FirstPosition :type Vector :default "0, 0, 0") (LastPosition :type Vector :default "0, 0, 0") (Factor :type Float%20%28single-precision%29))
  (bind (_x _y _z) (Math|Vector|BreakVector FirstPosition))
  (bind (_x_2 _y_2 _z_2) (Math|Vector|BreakVector LastPosition))
  (bind _returnvalue (- _x_2 _x))
  (bind _returnvalue_2 (- _y_2 _y))
  (bind _returnvalue_3 (- _z_2 _z))
  (bind _returnvalue_4 (* _returnvalue Factor))
  (bind _returnvalue_5 (* _returnvalue_2 Factor))
  (bind _returnvalue_6 (* _returnvalue_3 Factor))
  (bind _returnvalue_7 (Math|Vector|MakeVector _returnvalue_4 _returnvalue_5 _returnvalue_6))
  (Variables|Default|SetThrowingForce _returnvalue_7)
  (Development|PrintText (Utilities|Text|ToText(Float) (Math|Vector|VectorLength _returnvalue_7) "HalfToEven")))

(fn ObjectWayinHand
  (params (Hand :type EHands%20Enum :default "Left") (Player :type Kinect%20Character%20Object%20Reference))
  (bind _kinectmesh (Variables|/Game/Blueprints/KinectCharacter.KinectCharacter_C|GetKinectMesh Player))
  (if (== Hand 1)
    ;[1 1 1] Set Right Hand Positions Array
    (bind _outposition (Class|SkinnedMeshComponent|TransformfromBoneSpace _kinectmesh "middle_01_r" "0, 0, 0" "0, 0, 0"))
    (if (>= (Utilities|Array|Length (Variables|Default|GetHoldingHandPositionsRight)) 6)
      (bind _output_get (Variables|Default|SetThemporaryPositionsArray (Utilities|Array|MakeArray (Utilities|Array|Get(acopy) (Variables|Default|GetHoldingHandPositionsRight) 1) (Utilities|Array|Get(acopy) (Variables|Default|GetHoldingHandPositionsRight) 2) (Utilities|Array|Get(acopy) (Variables|Default|GetHoldingHandPositionsRight) 3) (Utilities|Array|Get(acopy) (Variables|Default|GetHoldingHandPositionsRight) 4) (Utilities|Array|Get(acopy) (Variables|Default|GetHoldingHandPositionsRight) 5) _outposition)))
      (Variables|Default|SetHoldingHandPositionsRight _output_get)
      (else
        (Utilities|Array|Add (Variables|Default|GetHoldingHandPositionsRight) _outposition)))
    (else
      ;[1 1 1] Set Left Hand Positions Array
      (bind _outposition_2 (Class|SkinnedMeshComponent|TransformfromBoneSpace _kinectmesh "None" "0, 0, 0" "0, 0, 0"))
      (if (>= (Utilities|Array|Length (Variables|Default|GetHoldingHandPositionsLeft)) 6)
        (bind _output_get_2 (Variables|Default|SetThemporaryPositionsArray (Utilities|Array|MakeArray (Utilities|Array|Get(acopy) (Variables|Default|GetHoldingHandPositionsLeft) 1) (Utilities|Array|Get(acopy) (Variables|Default|GetHoldingHandPositionsLeft) 2) (Utilities|Array|Get(acopy) (Variables|Default|GetHoldingHandPositionsLeft) 3) (Utilities|Array|Get(acopy) (Variables|Default|GetHoldingHandPositionsLeft) 4) (Utilities|Array|Get(acopy) (Variables|Default|GetHoldingHandPositionsLeft) 5) _outposition_2)))
        (Variables|Default|SetHoldingHandPositionsLeft _output_get_2)
        (else
          (Utilities|Array|Add (Variables|Default|GetHoldingHandPositionsLeft) _outposition_2)))))
  (return Player))